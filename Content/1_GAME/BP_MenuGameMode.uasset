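; BP_MenuGameMode is a game mode Blueprint that records bone pickups and drinking on the game instance.
; CollectBones adds the given value to the score and increments the count of bones collected.
; Drink sets hydration to the given value, replacing the previous one, and increments the count of water consumed.
; BeginPlay, Tick and the construction script are empty.
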(event EventBeginPlay)

(event EventTick
  (params (DeltaSeconds :type Float%20%28single-precision%29)))

(fn ConstructionScript)

(fn CollectBones
  (params (Valeur :type Integer))
  (bind _refbp_gameinstance (Variables|Default|GetRefBP_GameInstance))
  (Variables|/Game/1_GAME/BP_GameInstance.BP_GameInstance_C|SetScore _refbp_gameinstance (+ Valeur (Variables|/Game/1_GAME/BP_GameInstance.BP_GameInstance_C|GetScore _refbp_gameinstance)))
  (bind _result (Math|Integer|IncrementInt (Variables|/Game/1_GAME/BP_GameInstance.BP_GameInstance_C|GetOsRamasse _refbp_gameinstance))
    (:%20%20
      (Variables|/Game/1_GAME/BP_GameInstance.BP_GameInstance_C|SetOsRamasse _refbp_gameinstance _result))))

(fn Drink
  (params (Hydratation :type Float%20%28double-precision%29))
  (bind _refbp_gameinstance (Variables|Default|GetRefBP_GameInstance))
  (Variables|/Game/1_GAME/BP_GameInstance.BP_GameInstance_C|SetHydratation _refbp_gameinstance Hydratation)
  (bind _result (Math|Integer|IncrementInt (Variables|/Game/1_GAME/BP_GameInstance.BP_GameInstance_C|GetEauConsomme _refbp_gameinstance))
    (:%20%20
      (Variables|/Game/1_GAME/BP_GameInstance.BP_GameInstance_C|SetEauConsomme _refbp_gameinstance _result))))