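; Base Blueprint for food pickups that replenish the VR player's food value when collected.
; On BeginPlay it caches the game instance and the player's VRPawn through casts.
; Its Collect event adds a random amount between MinFood and MaxFood to the pawn's Food, then increments the game instance's NourritureConsomme counter of food consumed.
; Nothing in this graph calls Collect or destroys the actor.
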(event EventBeginPlay
  (bind _asbp_game_instance (Utilities|Casting|CastToBP_GameInstance (Game|GetGameInstance)))
  (Variables|Default|SetBP%20Game%20Instance _asbp_game_instance)
  (bind _asvrpawn (Utilities|Casting|CastToVRPawn (Game|Player|GetPlayerPawn 0)))
  (Variables|Default|SetVRPawn _asvrpawn))

(event EventTick
  (params (DeltaSeconds :type Float%20%28single-precision%29)))

(event EventCollect
  (bind _vrpawn (Variables|Default|GetVRPawn))
  (bind _bp_game_instance (Variables|Default|GetBP%20Game%20Instance))
  (Variables|/Game/1_GAME/Blueprints/VRPawn.VRPawn_C|SetFood _vrpawn (+ (Math|Random|RandomFloatinRange (Variables|Default|GetMinFood) (Variables|Default|GetMaxFood)) (Variables|/Game/1_GAME/Blueprints/VRPawn.VRPawn_C|GetFood _vrpawn)))
  (bind _result (Math|Integer|IncrementInt (Variables|/Game/1_GAME/BP_GameInstance.BP_GameInstance_C|GetNourritureConsomme _bp_game_instance))
    (:%20%20
      (Variables|/Game/1_GAME/BP_GameInstance.BP_GameInstance_C|SetNourritureConsomme _bp_game_instance _result))))

(fn ConstructionScript)