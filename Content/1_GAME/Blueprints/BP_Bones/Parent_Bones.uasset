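; Parent Blueprint for collectible bones that give a random value to the game mode when collected.
; BeginPlay casts the game mode to BP_GameMode and stores the reference.
; The Collect event rolls an integer between ValeurMin and ValeurMax, passes it to the game mode's CollectBones, then destroys the actor after a zero-length delay.
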(event EventBeginPlay
  (bind _asbp_game_mode (Utilities|Casting|CastToBP_GameMode (Game|GetGameMode)))
  (Variables|Default|SetRefBP_GameMode _asbp_game_mode))

(event EventTick
  (params (DeltaSeconds :type Float%20%28single-precision%29)))

(event EventCollect
  (bind _output_get (Variables|Default|SetValeur (Math|Random|RandomIntegerinRange (Variables|Default|GetValeurMin) (Variables|Default|GetValeurMax))))
  (Default|CollectBones (Variables|Default|GetRefBP_GameMode) _output_get)
  (Utilities|FlowControl|Delay 0.0)
  (Actor|DestroyActor))

(fn ConstructionScript)