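; Base Blueprint for collectible water that rehydrates the VR player when collected.
; On BeginPlay it caches the game instance and the VR pawn.
; Collect adds a random amount within a min/max range to the pawn's hydration, clamped to its valid range, increments the game instance's water-consumed counter, then destroys itself after a zero-length delay.
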(event EventBeginPlay
  (bind _asbp_game_instance (Utilities|Casting|CastToBP_GameInstance (Game|GetGameInstance)))
  (Variables|Default|SetBP%20Game%20Instance _asbp_game_instance)
  (bind _asvrpawn (Utilities|Casting|CastToVRPawn (Game|Player|GetPlayerPawn 0)))
  (Variables|Default|SetVRPawn _asvrpawn))

(event EventTick
  (params (DeltaSeconds :type Float%20%28single-precision%29)))

(event EventCollect
  (bind _vrpawn (Variables|Default|GetVRPawn))
  (bind _bp_game_instance (Variables|Default|GetBP%20Game%20Instance))
  (Variables|/Game/1_GAME/Blueprints/VRPawn.VRPawn_C|SetHydratation _vrpawn (Math|Float|Clamp(Float) (+ (Math|Random|RandomFloatinRange (Variables|Default|GetMinHydratation) (Variables|Default|GetMaxHydratation)) (Variables|/Game/1_GAME/Blueprints/VRPawn.VRPawn_C|GetHydratation _vrpawn)) 0.0 1e+02))
  (bind _result (Math|Integer|IncrementInt (Variables|/Game/1_GAME/BP_GameInstance.BP_GameInstance_C|GetEauConsomme _bp_game_instance))
    (:%20%20
      (Variables|/Game/1_GAME/BP_GameInstance.BP_GameInstance_C|SetEauConsomme _bp_game_instance _result)
      (Utilities|FlowControl|Delay 0.0)
      (Actor|DestroyActor))))

(fn ConstructionScript)