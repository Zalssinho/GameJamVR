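; Parent Blueprint for collectible water in a VR game, which sets the player's hydration when collected.
; BeginPlay caches references to the game instance and the VR pawn.
; Collect overwrites the pawn's Hydratation with a random value between the actor's min and max, rather than adding to it.
; It also increments the game instance's EauConsomme counter, then destroys the actor after a zero-length delay.
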(event EventBeginPlay
  (bind _asbp_game_instance (Utilities|Casting|CastToBP_GameInstance (Game|GetGameInstance)))
  (Variables|Default|SetBP%20Game%20Instance _asbp_game_instance)
  (bind _asvrpawn (Utilities|Casting|CastToVRPawn (Game|Player|GetPlayerPawn 0)))
  (Variables|Default|SetVRPawn _asvrpawn))

(event EventTick
  (params (DeltaSeconds :type Float%20%28single-precision%29)))

(event EventCollect
  (bind _bp_game_instance (Variables|Default|GetBP%20Game%20Instance))
  (Variables|/Game/1_GAME/Blueprints/VRPawn.VRPawn_C|SetHydratation (Variables|Default|GetVRPawn) (Math|Random|RandomFloatinRange (Variables|Default|GetMinHydratation) (Variables|Default|GetMaxHydratation)))
  (bind _result (Math|Integer|IncrementInt (Variables|/Game/1_GAME/BP_GameInstance.BP_GameInstance_C|GetEauConsomme _bp_game_instance))
    (:%20%20
      (Variables|/Game/1_GAME/BP_GameInstance.BP_GameInstance_C|SetEauConsomme _bp_game_instance _result)
      (Utilities|FlowControl|Delay 0.0)
      (Actor|DestroyActor))))

(fn ConstructionScript)