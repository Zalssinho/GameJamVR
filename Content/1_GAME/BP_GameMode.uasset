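; Game mode for a VR survival game that closes the game when the player's hydration or hunger (Faim) reaches zero.
; BeginPlay caches BP_GameInstance, which holds the stats, and the VR pawn, which is not otherwise used here.
; Tick polls both stats for exact zero and calls QuitGame directly.
; CollectBones and Drink overwrite the instance's Score and Hydratation with the passed value rather than adding to it.
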(event EventBeginPlay
  (bind _asbp_game_instance (Utilities|Casting|CastToBP_GameInstance (Game|GetGameInstance)))
  (Variables|Default|SetRefBP_GameInstance _asbp_game_instance)
  (bind _asvrpawn (Utilities|Casting|CastToVRPawn (Game|Player|GetPlayerPawn 0)))
  (Variables|Default|SetRefBP_VRPawn _asvrpawn))

(event EventTick
  (params (DeltaSeconds :type Float%20%28single-precision%29))
  (bind _refbp_gameinstance (Variables|Default|GetRefBP_GameInstance))
  (if (== (Variables|/Game/1_GAME/BP_GameInstance.BP_GameInstance_C|GetHydratation _refbp_gameinstance) 0.0)
    (Game|QuitGame 0 "Quit" false)
    (elif (== (Variables|/Game/1_GAME/BP_GameInstance.BP_GameInstance_C|GetFaim _refbp_gameinstance) 0.0)
      (Game|QuitGame 0 "Quit" false))))

(fn ConstructionScript)

(fn CollectBones
  (params (Valeur :type Integer))
  (Variables|/Game/1_GAME/BP_GameInstance.BP_GameInstance_C|SetScore (Variables|Default|GetRefBP_GameInstance) Valeur))

(fn Drink
  (params (Hydratation :type Float%20%28double-precision%29))
  (Variables|/Game/1_GAME/BP_GameInstance.BP_GameInstance_C|SetHydratation (Variables|Default|GetRefBP_GameInstance) Hydratation))